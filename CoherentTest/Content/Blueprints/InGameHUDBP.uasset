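; In-game Cohtml HUD Blueprint that shows an HTML page for spawning, destroying and counting TopDownNPCs.
; BeginPlay loads the page and ensures a mouse-accepting CohtmlInputActor exists; CreateModel registers the NPCInfoModel data model.
; A fast looping timer runs UpdateModel, pushing live count, portal spawn count and screen-projected NPC labels.
; Button events spawn through the first NPCPortal, destroy all NPCs or adjust the clamped spawn count.
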(event EventBeginPlay
  (Class|CohtmlGameHUD|SetupView "coui://uiresources/GameHUD/HUD.html" true false)
  (CallFunction|SetupinGameInput)
  (EventDispatchers|BindEventtoReadyforBindings (Variables|Default|GetCohtmlHUD) (EventDispatchers|CreateEvent :!event CreateModel)))

(event Collision|EventActorBeginOverlap
  (params (OtherActor :type Actor%20Object%20Reference)))

(event EventOnGenerateBtnClicked
  (bind _outactors (Actor|GetAllActorsOfClass "/Game/Blueprints/NPCPortal.NPCPortal_C"))
  (Default|SpawnNPC (Utilities|Array|Get(acopy) _outactors))
  (CallFunction|UpdateModel))

(event EventOnDestroyBtnClicked
  (bind _outactors (Actor|GetAllActorsOfClass "/Game/TopDownBP/Blueprints/TopDownNPC.TopDownNPC_C"))
  (for _array_element _outactors
    (Actor|DestroyActor _array_element)
    (CallFunction|UpdateModel)))

(event EventOnSliderBtnClicked
  (params (val :type String))
  (CallFunction|AddtoSliderVal (Math|Conversions|ToInteger(Byte) val)))

(fn ConstructionScript)

(fn SetupinGameInput
  (bind _outactors (Actor|GetAllActorsOfClass "/Script/CohtmlPlugin.CohtmlInputActor"))
  (if (== (Utilities|Array|Length _outactors) 0)
    (bind _returnvalue (Game|SpawnActorfromClass "/Script/CohtmlPlugin.CohtmlInputActor" (Math|Transform|MakeTransform "0, 0, 0") "AdjustIfPossibleButDontSpawnIfColliding" 0 0))
    (Class|CohtmlInputActor|Initialize _returnvalue "ECC_WorldDynamic" "TA_Wrap" "CohtmlRaycastQuality_Accurate")
    (Class|CohtmlInputActor|AlwaysAcceptMouseInput _returnvalue true)
    (return)))

(fn GetCurrentNPCsCount
  (bind _outactors (Actor|GetAllActorsOfClass "/Game/TopDownBP/Blueprints/TopDownNPC.TopDownNPC_C"))
  (return (Utilities|Array|Length _outactors)))

(fn GetNPCCounttoGenerete
  (bind _outactors (Actor|GetAllActorsOfClass "/Game/Blueprints/NPCPortal.NPCPortal_C"))
  (return (Variables|/Game/Blueprints/NPCPortal.NPCPortal_C|GetNPCCount (Utilities|Array|Get(acopy) _outactors))))

(fn GetActorsInfo
  (bind _outactors (Actor|GetAllActorsOfClass "/Game/TopDownBP/Blueprints/TopDownNPC.TopDownNPC_C"))
  (for _array_element _outactors
    (bind _output_get (LocalVariables|SetNPC _array_element))
    (Utilities|Array|Add (LocalVariables|GetActors) (Utilities|Struct|MakeActorInfo (Utilities|GetDisplayName _output_get) (- (.Y (Math|Vector2D|BreakVector2D (.ScreenLocation (Class|PlayerController|ProjectWorldLocationtoScreen (Game|GetPlayerController 0) (Transformation|GetActorLocation _output_get) false)))) 5e+01) (- (.X (Math|Vector2D|BreakVector2D (.ScreenLocation (Class|PlayerController|ProjectWorldLocationtoScreen (Game|GetPlayerController 0) (Transformation|GetActorLocation _output_get) false)))) 5e+01))))
  (return (LocalVariables|GetActors)))

(fn UpdateModel
  (bind _returnvalue (CallFunction|GetCurrentNPCsCount))
  (bind _npccount (CallFunction|GetNPCCounttoGenerete))
  (bind _actors1 (CallFunction|GetActorsInfo))
  (bind _output_get (Variables|Default|SetnpcInfo (Utilities|Struct|MakeNPCInfo _returnvalue _npccount _actors1)))
  (bind _asprysm_gamehud (Utilities|Casting|CastToCohtmlGameHUD (HUD|GetHUD (Game|GetPlayerController 0))))
  (Class|CohtmlBaseComponent|UpdateWholeDataModelfromStruct (Variables|/Script/CohtmlPlugin.CohtmlGameHUD|GetCohtmlHUD _asprysm_gamehud) _output_get)
  (Class|CohtmlBaseComponent|SynchronizeModels (Variables|/Script/CohtmlPlugin.CohtmlGameHUD|GetCohtmlHUD _asprysm_gamehud)))

(fn CreateModel
  (bind _npcinfo (Variables|Default|GetnpcInfo))
  (bind _asprysm_gamehud (Utilities|Casting|CastToCohtmlGameHUD (HUD|GetHUD (Game|GetPlayerController 0))))
  (Class|CohtmlBaseComponent|CreateDataModelfromStruct (Variables|/Script/CohtmlPlugin.CohtmlGameHUD|GetCohtmlHUD _asprysm_gamehud) "NPCInfoModel" _npcinfo)
  (Class|CohtmlBaseComponent|UpdateWholeDataModelfromStruct (Variables|/Script/CohtmlPlugin.CohtmlGameHUD|GetCohtmlHUD _asprysm_gamehud) _npcinfo)
  (Class|CohtmlBaseComponent|SynchronizeModels (Variables|/Script/CohtmlPlugin.CohtmlGameHUD|GetCohtmlHUD _asprysm_gamehud))
  (Utilities|Time|SetTimerbyFunctionName 0 "UpdateModel" 0.01 true))

(fn AddtoSliderVal
  (params (ValueToAdd :type Integer))
  (bind _outactors (Actor|GetAllActorsOfClass "/Game/Blueprints/NPCPortal.NPCPortal_C"))
  (Variables|/Game/Blueprints/NPCPortal.NPCPortal_C|SetNPCCount (Utilities|Array|Get(acopy) _outactors) (Math|Integer|Clamp(Integer) (+ ValueToAdd (.npcgeneratecount (Variables|Default|GetnpcInfo))) 1 100))
  (CallFunction|UpdateModel))