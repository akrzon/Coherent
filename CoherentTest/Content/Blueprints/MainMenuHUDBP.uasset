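; Main menu HUD Blueprint that shows an HTML menu through Coherent Gameface (Cohtml) and handles its Start and Quit buttons.
; BeginPlay loads the MainMenu page with complex CSS support, then spawns and initializes a CohtmlInputActor set to always accept mouse input if none exists.
; The Start handler opens the TopDownExampleMap level, and the Quit handler runs the quit console command.
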(event EventBeginPlay
  (Class|CohtmlGameHUD|SetupView "coui://uiresources/MainMenuHUD/MainMenu.html" true false)
  (CallFunction|SetupInput))

(event Collision|EventActorBeginOverlap
  (params (OtherActor :type Actor%20Object%20Reference)))

(event EventTick
  (params (DeltaSeconds :type Float%20%28single-precision%29)))

(event EventOnQuitBtnClicked
  (Development|ExecuteConsoleCommand "quit" 0))

(event EventOnStartBtnClicked
  (Game|OpenLevel(byName) "TopDownExampleMap"))

(fn ConstructionScript)

(fn SetupInput
  (bind _outactors (Actor|GetAllActorsOfClass "/Script/CohtmlPlugin.CohtmlInputActor"))
  (if (== (Utilities|Array|Length _outactors) 0)
    (bind _returnvalue (Game|SpawnActorfromClass "/Script/CohtmlPlugin.CohtmlInputActor" (Math|Transform|MakeTransform "0, 0, 0") "AdjustIfPossibleButDontSpawnIfColliding" 0 0))
    (Class|CohtmlInputActor|Initialize _returnvalue "ECC_WorldDynamic" "TA_Wrap" "CohtmlRaycastQuality_Accurate")
    (Class|CohtmlInputActor|AlwaysAcceptMouseInput _returnvalue true)
    (return)))